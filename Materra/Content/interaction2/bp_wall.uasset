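; Interactable wall actor that shows an outline when the third-person character overlaps it and is destroyed on interaction.
; Begin overlap casts to BP_ThirdPersonCharacter and sets M_outline as the static mesh's overlay material, while any end overlap clears it.
; The Interaction event destroys the actor, and an unconnected CameraBoom arm-length setter never runs.
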(event Collision|EventActorEndOverlap
  (params (OtherActor :type Actor%20Object%20Reference))
  (Rendering|Material|SetOverlayMaterial (Variables|Default|GetStaticMesh) 0 :!class /Script/Engine.MeshComponent))

(event Collision|EventActorBeginOverlap
  (params (OtherActor :type Actor%20Object%20Reference))
  (Utilities|Casting|CastToBP_ThirdPersonCharacter OtherActor)
  (Rendering|Material|SetOverlayMaterial (Variables|Default|GetStaticMesh) "/Game/interaction2/m_outline.m_outline" :!class /Script/Engine.MeshComponent))

(event EventInteraction
  (Actor|DestroyActor))

(fn ConstructionScript
  (|CallParentFunction))