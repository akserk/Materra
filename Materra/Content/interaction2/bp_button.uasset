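; Interactable button actor that shows an outline overlay material while the third-person character overlaps it and shrinks when interacted with.
; Begin overlap applies the outline only for that character, while any end overlap clears it.
; The Interaction event sets a flag that makes Tick interpolate the actor's scale toward zero, until a one-second delay clears the flag.
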(event Collision|EventActorEndOverlap
  (params (OtherActor :type Actor%20Object%20Reference))
  (Rendering|Material|SetOverlayMaterial (Variables|Default|GetStaticMesh) 0 :!class /Script/Engine.MeshComponent))

(event Collision|EventActorBeginOverlap
  (params (OtherActor :type Actor%20Object%20Reference))
  (Utilities|Casting|CastToBP_ThirdPersonCharacter OtherActor)
  (Rendering|Material|SetOverlayMaterial (Variables|Default|GetStaticMesh) "/Game/interaction2/m_outline.m_outline" :!class /Script/Engine.MeshComponent))

(event EventInteraction
  (bind _output_get (Variables|Default|Setinteracting true)))

(event EventTick
  (params (DeltaSeconds :type Float%20%28single-precision%29))
  (if (stale EventInteraction _output_get)
    (Transformation|SetActorScale3D (Math|Interpolation|VInterpTo (Transformation|GetActorScale3D) "0, 0, 0" (Utilities|Time|GetWorldDeltaSeconds) 3.0))
    (Utilities|FlowControl|Delay 1.0)
    (Variables|Default|Setinteracting false)))

(fn ConstructionScript
  (|CallParentFunction))