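; Actor component that detects which interaction area the player camera is looking at and toggles that area's focus.
; Every tick it runs a debug-drawn Visibility line trace forward from the camera over a set length.
; When the hit actor changes, an exact class match to Bp_interact_area moves focus to it, unfocusing any previous area.
; A miss or different class releases the currently focused area.
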(event EventTick
  (params (DeltaSeconds :type Float%20%28single-precision%29))
  (CallFunction|Trace))

(fn Trace
  (bind _returnvalue (Game|GetPlayerCameraManager 0))
  (bind _returnvalue_2 (Transformation|GetActorLocation _returnvalue))
  (bind (_outhit _returnvalue_3) (Collision|LineTraceByChannel _returnvalue_2 (+ _returnvalue_2 (* (Math|Vector|GetForwardVector (Transformation|GetActorRotation _returnvalue)) (Variables|Default|Getlength))) "TraceTypeQuery1" false 0 "ForDuration"))
  (if _returnvalue_3
    (if (!= (Variables|Default|Getfocused_actor) (.HitActor (Collision|BreakHitResult _outhit)))
      (Variables|Default|Setfocused_actor (.HitActor (Collision|BreakHitResult _outhit)))
      (CallFunction|Traceinteractionarea (== (Utilities|GetClass (.HitActor (Collision|BreakHitResult _outhit))) "/Game/interaction2/interaction_area/bp_interact_area.bp_interact_area_C")))
    (else
      (CallFunction|Traceinteractionarea false))))

(fn Traceinteractionarea
  (params (trace :type Boolean))
  (if trace
    (if (Variables|Default|Getis_tracing_into_actionarea)
      (Default|ToggleFocus (Variables|Default|Getfocused_interaction_area) false))
    (bind _asbp_interact_area (Utilities|Casting|CastTobp_interact_area (Variables|Default|Getfocused_actor)))
    (bind _output_get (Variables|Default|Setfocused_interaction_area _asbp_interact_area))
    (Default|ToggleFocus _output_get true)
    (Variables|Default|Setis_tracing_into_actionarea true)
    (elif (Variables|Default|Getis_tracing_into_actionarea)
      (Variables|Default|Setis_tracing_into_actionarea false)
      (Default|ToggleFocus (Variables|Default|Getfocused_interaction_area) false)
      (Variables|Default|Setfocused_actor 0)
      (Variables|Default|Setfocused_interaction_area 0))))