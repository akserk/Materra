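; bp_button1 is an interactable button that highlights with an outline overlay material while an actor overlaps it.
; Interaction sets a flag, and Tick then interpolates the second mesh toward full scale.
; After a one-second Delay it clears the flag, sets Placed and adds a half-turn to the player character if it casts to bp_MATERA_housemap, otherwise printing debug text.
; A separate Placed-based rotation branch is left unconnected.
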(event Custom|CustomEvent)

(event Collision|EventActorEndOverlap
  (params (OtherActor :type Actor%20Object%20Reference))
  (Rendering|Material|SetOverlayMaterial (Variables|Default|GetStaticMesh) 0 :!class /Script/Engine.MeshComponent))

(event Collision|EventActorBeginOverlap
  (params (OtherActor :type Actor%20Object%20Reference))
  (Rendering|Material|SetOverlayMaterial (Variables|Default|GetStaticMesh) "/Game/interaction2/m_outline.m_outline" :!class /Script/Engine.MeshComponent))

(event EventInteraction
  (bind _output_get (Variables|Default|Setinteracted true)))

(event EventTick
  (params (DeltaSeconds :type Float%20%28single-precision%29))
  (if (stale EventInteraction _output_get)
    (Transformation|SetRelativeScale3D (Variables|Default|GetStaticMesh1) (Math|Interpolation|VInterpTo (Transformation|GetWorldScale (Variables|Default|GetStaticMesh1)) "1.000000,1.000000,1.000000" (Utilities|Time|GetWorldDeltaSeconds) 1e+01))
    (Utilities|FlowControl|Delay 1.0)
    (Variables|Default|Setinteracted false)
    (Variables|Default|Setplaced true)
    (bind _asbp_matera_housemap (Utilities|Casting|CastTobp_MATERA_housemap (Game|GetPlayerCharacter 0))
      (:then
        (Transformation|AddWorldRotation (Variables|/Script/Engine.Actor|GetRootComponent _asbp_matera_housemap) "0.000000,180.000000,0.000000" false false))
      (:CastFailed
        (Development|PrintString "Hello")))))

(fn ConstructionScript
  (|CallParentFunction))