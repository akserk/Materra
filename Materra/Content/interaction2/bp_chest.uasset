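; Interactable chest actor that toggles between open and closed when its Interaction event fires.
; Interaction plays the opening or closing skeletal animation, flips the Closed flag and blocks retriggering for a one-second delay.
; Overlap with BP_ThirdPersonCharacter applies an outline overlay material while the chest is closed, and any end overlap clears it.
; Disconnected debug and older key-press logic remains in the graph but never runs.
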(event Collision|EventActorEndOverlap
  (params (OtherActor :type Actor%20Object%20Reference))
  (Rendering|Material|SetOverlayMaterial (Variables|Default|GetSkeletalMesh) 0 :!class /Script/Engine.MeshComponent))

(event Collision|EventActorBeginOverlap
  (params (OtherActor :type Actor%20Object%20Reference))
  (if (Variables|Default|Getclosed)
    (Utilities|Casting|CastToBP_ThirdPersonCharacter OtherActor)
    (Rendering|Material|SetOverlayMaterial (Variables|Default|GetSkeletalMesh) "/Game/interaction2/m_outline.m_outline" :!class /Script/Engine.MeshComponent)))

(event EventInteraction
  (if (not (Variables|Default|Getinproccess))
    (if (Variables|Default|Getclosed)
      (Variables|Default|Setinproccess true)
      (Components|Animation|PlayAnimation (Variables|Default|GetSkeletalMesh) "/Game/other/opening.opening" false)
      (Variables|Default|Setclosed false)
      (Utilities|FlowControl|Delay 1.0)
      (Variables|Default|Setinproccess false)
      (else
        (Variables|Default|Setinproccess true)
        (Components|Animation|PlayAnimation (Variables|Default|GetSkeletalMesh) "/Game/other/closing.closing" false)
        (Variables|Default|Setclosed true)
        (Utilities|FlowControl|Delay 1.0)
        (Variables|Default|Setinproccess false)))))

(fn ConstructionScript
  (|CallParentFunction))