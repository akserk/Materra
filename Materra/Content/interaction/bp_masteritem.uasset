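; Base interactable item actor that shows a hint and outline when the third-person character comes into range.
; While CanInteract is set, sphere overlap creates a widget, plays its popup animation, applies an overlay outline and enables CanPressE.
; Leaving clears these and removes the widget after a short delay.
; CanRecieveTrace also toggles the hint; the E press itself is not handled here.
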(event OnComponentBeginOverlap(Sphere)
  (params (OverlappedComponent :type Primitive%20Component%20Object%20Reference) (OtherActor :type Actor%20Object%20Reference) (OtherComp :type Primitive%20Component%20Object%20Reference) (OtherBodyIndex :type Integer) (bFromSweep :type Boolean) (SweepResult :type Hit%20Result%20Structure%20%28by%20ref%29))
  (bind _widget (Variables|Default|GetWidget))
  (Utilities|Casting|CastToBP_ThirdPersonCharacter OtherActor)
  (if (Variables|Default|Getcan_interact)
    (bind _returnvalue (UserInterface|CreateWidget "/Game/interaction/ui_interact.ui_interact_C"))
    (bind _output_get (Variables|Default|Setinteraction_widget _returnvalue))
    (UserInterface|SetWidget _widget _output_get)
    (Rendering|SetVisibility _widget true false)
    (bind _interaction_widget (Variables|Default|Getinteraction_widget)
      (:then
        (if (not (Variables|Default|Gethint_visible))
          (UserInterface|Animation|PlayAnimation _interaction_widget (Variables|/Game/interaction/ui_interact.ui_interact_C|Getpopup _interaction_widget) 0.0 1 "Forward" 1.5 false)
          (Variables|Default|Sethint_visible true)
          (Rendering|Material|SetOverlayMaterial (Variables|Default|GetStaticMesh) "/Game/interaction/m_outline.m_outline" :!class /Script/Engine.MeshComponent)
          (Variables|Default|Setcan_press_e true)))
      (:else))))

(event OnComponentEndOverlap(Sphere)
  (params (OverlappedComponent :type Primitive%20Component%20Object%20Reference) (OtherActor :type Actor%20Object%20Reference) (OtherComp :type Primitive%20Component%20Object%20Reference) (OtherBodyIndex :type Integer))
  (Utilities|Casting|CastToBP_ThirdPersonCharacter OtherActor)
  (if (Variables|Default|Getcan_interact)
    (bind _interaction_widget (Variables|Default|Getinteraction_widget)
      (:then
        (if (Variables|Default|Gethint_visible)
          (UserInterface|Animation|PlayAnimation _interaction_widget (Variables|/Game/interaction/ui_interact.ui_interact_C|Getpopup _interaction_widget) 0.0 1 "Forward" 1.5 false)
          (Variables|Default|Sethint_visible false)
          (Variables|Default|Setcan_press_e false)
          (Rendering|Material|SetOverlayMaterial (Variables|Default|GetStaticMesh) 0 :!class /Script/Engine.MeshComponent))
        (Utilities|FlowControl|Delay 0.15)
        (Widget|RemovefromParent (Variables|Default|Getinteraction_widget))
        (Variables|Default|Setinteraction_widget 0)
        (Rendering|SetVisibility (Variables|Default|GetWidget) false false))
      (:else))))

(event EventCanRecieveTrace
  (params (can_interact :type Boolean))
  (if (Variables|Default|Getcan_interact)
    (if can_interact
      (bind _interaction_widget (Variables|Default|Getinteraction_widget)
        (:then
          (if (not (Variables|Default|Gethint_visible))
            (UserInterface|Animation|PlayAnimation _interaction_widget (Variables|/Game/interaction/ui_interact.ui_interact_C|Getpopup _interaction_widget) 0.0 1 "Forward" 1.5 false)
            (Variables|Default|Sethint_visible true)
            (Rendering|Material|SetOverlayMaterial (Variables|Default|GetStaticMesh) "/Game/interaction/m_outline.m_outline" :!class /Script/Engine.MeshComponent)
            (Variables|Default|Setcan_press_e true)))
        (:else))
      (else
        (bind _interaction_widget_2 (Variables|Default|Getinteraction_widget)
          (:then
            (if (Variables|Default|Gethint_visible)
              (UserInterface|Animation|PlayAnimation _interaction_widget_2 (Variables|/Game/interaction/ui_interact.ui_interact_C|Getpopup _interaction_widget_2) 0.0 1 "Reverse" 1.5 false)
              (Variables|Default|Sethint_visible false)
              (Rendering|Material|SetOverlayMaterial (Variables|Default|GetStaticMesh) 0 :!class /Script/Engine.MeshComponent)
              (Variables|Default|Setcan_press_e false)))
          (:else))))))

(fn ConstructionScript)