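; Chest Blueprint with an Interaction event meant to play an animation on its skeletal mesh.
; Interaction requires CanPressE and CanInteract, prints a debug string, then clears CanInteract.
; It then tests CanInteract again before the looping animation, so that branch fails as written.
; The overlap event is empty, and several other animation nodes are left unconnected.
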(event Collision|EventActorBeginOverlap
  (params (OtherActor :type Actor%20Object%20Reference)))

(event EventInteraction
  (bind _can_press_e (Variables|Default|Getcan_press_e))
  (if _can_press_e
    (if (Variables|Default|Getcan_interact)
      (Development|PrintString (Utilities|String|ToString(Boolean) _can_press_e))
      (bind _output_get (Variables|Default|Setcan_interact false))
      (if _output_get
        (Development|PrintString "Hello")
        (Components|Animation|PlayAnimation (Variables|Default|GetMATERA_chest) "/Game/other/MATERA_chest_Anim.MATERA_chest_Anim" true)))))

(fn ConstructionScript
  (|CallParentFunction))